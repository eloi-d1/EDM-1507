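; MIDI manager Blueprint that turns input from a MIDI controller into polyphonic MetaSound synth playback.
; On BeginPlay it opens the input device matching MIDIControllerIndex and binds its MIDI events.
; Each Note On spawns and plays an MSS_polysynth sound, stored in PolyVoices by note number so Note Off can trigger its release.
; A monosynth is created but never played, and its CC-to-parameter mapping is left unwired.
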(event Custom|Event%20on%20MIDI
  (params (MIDIDeviceController :type MIDI%20Device%20Controller%20Object%20Reference) (Timestamp :type Integer) (EventType :type EMIDIEventType%20Enum :default "Unknown") (Channel :type Integer) (ControlID :type Integer) (Velocity :type Integer) (RawEventType :type Integer))
  (bind _returnvalue (Math|Conversions|ToFloat(Integer) ControlID))
  (bind _returnvalue_2 (Math|Float|Truncate _returnvalue))
  (Development|PrintString (Utilities|String|ToString(Text) (Utilities|Text|FormatText "MIDI EVENT TYPE{event} MIDI Note{note} VELOCITE{velocite}" ControlID Velocity (Utilities|String|EnumtoString EventType))) true true "(R=0.000000,G=0.660000,B=1.000000,A=1.000000)" 2.0 "MIDI")
  (switch Utilities|FlowControl|Switch|SwitchonEMIDIEventType EventType
    (:NoteOff
      (Class|AudioParameterControllerInterface|SetTriggerParameter (Utilities|Array|Get(acopy) (Variables|Default|GetPoly%20voices) _returnvalue_2) "Trigger Release 1"))
    (:NoteOn
      (bind _returnvalue_3 (Audio|CreateSound2D "/Game/metasound/MSS_polysynth.MSS_polysynth" 1.0 1.0 0.0 0))
      (Utilities|Array|SetArrayElem (Variables|Default|GetPoly%20voices) _returnvalue_2 _returnvalue_3 true)
      (Audio|Parameter|SetFloatParameter _returnvalue_3 "MIDInote" _returnvalue :!class /Script/AudioExtensions.AudioParameterControllerInterface)
      (Audio|Components|Audio|Play _returnvalue_3 0.0))))

(event EventBeginPlay
  (bind _outmididevices (Class|MIDIDeviceManager|FindMIDIDevices))
  (for _array_element _outmididevices
    (if (.bCanReceiveFrom (Utilities|Struct|BreakFoundMIDIDevice _array_element))
      (if (== (Variables|Default|GetMIDI_controller_index) (.DeviceID (Utilities|Struct|BreakFoundMIDIDevice _array_element)))
        (Development|PrintString (.DeviceName (Utilities|Struct|BreakFoundMIDIDevice _array_element)) true true "(R=0.000000,G=0.660000,B=1.000000,A=1.000000)" 3e+01)
        (bind _returnvalue (Class|MIDIDeviceManager|CreateMIDIDeviceController (.DeviceID (Utilities|Struct|BreakFoundMIDIDevice _array_element)) 1024))
        (bind _output_get (Variables|Default|SetNewVar _returnvalue))
        (EventDispatchers|BindEventtoOnMIDIEvent _output_get (EventDispatchers|CreateEvent :!event Custom|Event%20on%20MIDI)))))
  (Development|PrintString "boucle terminer" true true "(R=0.000000,G=0.660000,B=1.000000,A=1.000000)" 3e+01)
  (bind _returnvalue_2 (Audio|CreateSound2D "/Game/metasound/MSS_monosynth.MSS_monosynth" 1.0 1.0 0.0 0))
  (Variables|Default|SetNewVar_0 _returnvalue_2))

(fn ConstructionScript)